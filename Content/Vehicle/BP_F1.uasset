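; BP_F1 is a player-driven Formula 1 vehicle Blueprint that maps input to driving and camera control.
; Throttle, brake and steer axes feed straight into the vehicle movement component.
; A FlipFlop on the ChangeCamera action toggles which of the onboard and spring-arm-era C++-named cameras is active.
; LookRight and LookUp share one node that adds relative pitch and yaw to the spring arm.
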(event `InputAxis|Brake`
  (params (AxisValue :type "Float (single-precision)"))
  (`ChaosVehicleMovementComponent.SetBrakeInput` (`self.VehicleMovementComponent`) AxisValue))

(event `InputAction|ChangeCamera`
  (params (Key :type "Key Structure"))
  (:`Pressed`
    (bind _isa (`/Engine/EditorBlueprintResources/StandardMacros.FlipFlop`)
      (:`A`
        _)
      (:`B`
        _))
    (`ActorComponent.SetActive` (`self.OnboardCameraCpp`) _isa false)
    (`ActorComponent.SetActive` (`self.CameraCpp`) (not _isa) false)))

(event `InputAxis|Throttle`
  (params (AxisValue :type "Float (single-precision)"))
  (`ChaosVehicleMovementComponent.SetThrottleInput` (`self.VehicleMovementComponent`) AxisValue))

(event `InputAxis|LookRight`
  (params (AxisValue :type "Float (single-precision)"))
  (`SceneComponent.K2_AddRelativeRotation` (`self.SpringArmCpp`) (`KismetMathLibrary.MakeRotator` 0.0 (stale `InputAxis|LookUp` AxisValue) AxisValue) false false :!label _label))

(event `InputAxis|Steer`
  (params (AxisValue :type "Float (single-precision)"))
  (`ChaosVehicleMovementComponent.SetSteeringInput` (`self.VehicleMovementComponent`) AxisValue))

(event `InputAxis|LookUp`
  (params (AxisValue :type "Float (single-precision)"))
  (goto _label))

(fn `UserConstructionScript`)